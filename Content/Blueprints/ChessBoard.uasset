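; ChessBoard is an actor Blueprint that builds an 8x8 checkered board of static mesh tiles in its construction script.
; Nested loops add one mesh component per square, spaced on a flat grid by the Offset variable.
; Comparing the parity of row and column indices assigns each tile the LightTile or DarkTile material.
; The event graph holds only disabled placeholder events, so the asset has no runtime logic.
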(event EventBeginPlay)

(event Collision|EventActorBeginOverlap
  (params (OtherActor :type Actor%20Object%20Reference)))

(event EventTick
  (params (DeltaSeconds :type Float%20%28single-precision%29)))

(fn ConstructionScript
  (bind _offset (LocalVariables|GetOffset))
  ;[1 1 1] 8x8 board
  (for _index (range 0 7)
    (for _index_2 (range 0 7)
      ;[1 1 1] mesh + material
      (bind _returnvalue (AddComponent|AddStaticMeshComponent false (Math|Conversions|ToTransform(Vector) (Math|Vector|MakeVector (* _index_2 _offset) (* _index _offset) 0.0))))
      (Rendering|Material|SetMaterial _returnvalue 0 (select (== (Math|Integer|%(Integer) _index_2 2) (Math|Integer|%(Integer) _index 2)) "/Game/Materials/LightTile.LightTile" "/Game/Materials/DarkTile.DarkTile")))))